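; BP_Track is a track Blueprint that changes its look to match a rain, snow or desert environment.
; Each environment event swaps the materials on the GroundPlane and TrackType components, with rain and desert sharing the standard track material.
; A separate SetTrack event assigns the basic track mesh to TrackType unless IsCustom is set.
; The construction script is empty, so all changes depend on these events being called.
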(event `Set Environment Rain`
  (`PrimitiveComponent.SetMaterial` (`self.Ground Plane`) 0 "/Game/Textures/Instances/MI_Grass.MI_Grass")
  (`PrimitiveComponent.SetMaterial` (`self.Track Type`) 0 "/Game/Textures/Instances/MI_Track.MI_Track"))

(event `Set Environment Snow`
  (`PrimitiveComponent.SetMaterial` (`self.Ground Plane`) 0 "/Game/Textures/Instances/MI_Ice.MI_Ice")
  (`PrimitiveComponent.SetMaterial` (`self.Track Type`) 0 "/Game/Textures/Instances/MI_Track_Snow.MI_Track_Snow"))

(event `Set Environment Desert`
  (`PrimitiveComponent.SetMaterial` (`self.Ground Plane`) 0 "/Game/Textures/Instances/MI_Sand.MI_Sand")
  (`PrimitiveComponent.SetMaterial` (`self.Track Type`) 0 "/Game/Textures/Instances/MI_Track.MI_Track"))

(event `Set Track`
  (if (not (`self.isCustom`))
    (`StaticMeshComponent.SetStaticMesh` (`self.Track Type`) "/Game/Mesh/SM_Basic_Track.SM_Basic_Track")))

(fn `UserConstructionScript`)