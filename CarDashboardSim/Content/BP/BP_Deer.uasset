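; BP_Deer is a deer actor that travels along its Direction variable and removes itself after a short lifetime.
; Each Tick moves the actor from the Deer component's world transform at a frame-rate-scaled speed, re-randomized every frame, with a yaw offset applied to that component's rotation.
; The same Tick chain runs a Delay before DestroyActor, so the first call starts the despawn countdown.
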(event `self.ReceiveTick`
  (params (DeltaSeconds :type "Float (single-precision)"))
  (bind _returnvalue (`SceneComponent.K2_GetComponentToWorld` (`self.Deer`)))
  (`self.K2_SetActorTransform` (`KismetMathLibrary.MakeTransform` (+ (* (`KismetMathLibrary.Normal` (`self.Direction`)) (* (`GameplayStatics.GetWorldDeltaSeconds`) (`KismetMathLibrary.RandomFloatInRange` 800.0 1300.0))) (.location _returnvalue)) (`KismetMathLibrary.MakeRotator` (.roll (.rotation _returnvalue)) (.pitch (.rotation _returnvalue)) (- (.yaw (.rotation _returnvalue)) 90.0)) (.scale _returnvalue)))
  (`KismetSystemLibrary.Delay` 15.0)
  (`self.K2_DestroyActor`))

(fn `UserConstructionScript`)