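; Dashboard gauge that acts as a tachometer, fuel gauge or MPH speedometer based on the IsRPM and IsFuel flags.
; Each tick it sets the face material, needle roll and text readout for its mode, reading the player's BP_Dashboard character.
; RPM derives from ground speed, a per-gear ratio and wheel diameter, then feeds back to the dashboard.
; Fuel drains a fixed step per tick, not scaled by delta time, and flags FuelEmpty at exactly zero.
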(event `self.ReceiveTick`
  (params (DeltaSeconds :type "Float (single-precision)"))
  (bind _sm_dial (`self.SM_Dial`))
  (bind _fuelamount (`self.fuelAmount`))
  (bind (_returnvalue_roll _returnvalue_pitch _returnvalue_yaw) (`KismetMathLibrary.BreakRotator` (`SceneComponent.K2_GetComponentRotation` _sm_dial)))
  (bind _asbp_dashboard (cast `/Game/BP/BP_Dashboard` (`GameplayStatics.GetPlayerCharacter` 0)))
  (if (`self.isRPM`)
    (`PrimitiveComponent.SetMaterial` (`self.SM_Dial_Base`) 0 "/Game/Textures/Instances/MI_Dial_RPM.MI_Dial_RPM")
    (switch `int` (`/Game/BP/BP_Dashboard.gear` _asbp_dashboard)
      (:`1`
        (bind _output_get (set `self.gearRatio` 14.25))
        (set `/Game/BP/BP_Dashboard.gearRatio` _output_get _asbp_dashboard))
      (:`2`
        (bind _output_get_2 (set `self.gearRatio` 8.21))
        (set `/Game/BP/BP_Dashboard.gearRatio` _output_get_2 _asbp_dashboard))
      (:`3`
        (bind _output_get_3 (set `self.gearRatio` 5.67))
        (set `/Game/BP/BP_Dashboard.gearRatio` _output_get_3 _asbp_dashboard))
      (:`4`
        (bind _output_get_4 (set `self.gearRatio` 4.55))
        (set `/Game/BP/BP_Dashboard.gearRatio` _output_get_4 _asbp_dashboard))
      (:`5`
        (bind _output_get_5 (set `self.gearRatio` 3.8))
        (set `/Game/BP/BP_Dashboard.gearRatio` _output_get_5 _asbp_dashboard))
      (:`6`
        (bind _output_get_6 (set `self.gearRatio` 3.13))
        (set `/Game/BP/BP_Dashboard.gearRatio` _output_get_6 _asbp_dashboard)))
    (bind _returnvalue (/ (`KismetMathLibrary.VSizeXY` (`MovementComponent.Velocity` (`Character.CharacterMovement` _asbp_dashboard))) 44.704))
    (bind _returnvalue_2 (/ (* _returnvalue (`self.gearRatio`) 336.0) (`/Game/BP/BP_Dashboard.wheelDiameter` _asbp_dashboard)))
    (`SceneComponent.K2_SetWorldRotation` _sm_dial (`KismetMathLibrary.MakeRotator` (`KismetMathLibrary.MapRangeClamped` _returnvalue_2 0.0 8000.0 -110.0 110.0) _returnvalue_pitch _returnvalue_yaw) false false)
    (bind _returnvalue_3 (`KismetMathLibrary.Round64` (/ _returnvalue_2 1000.0)))
    (`TextRenderComponent.K2_SetText` (`self.TextRender`) (`KismetTextLibrary.Conv_Int64ToText` _returnvalue_3))
    (set `/Game/BP/BP_Dashboard.RPM` (`KismetMathLibrary.Conv_Int64ToInt` _returnvalue_3) _asbp_dashboard)
    (set `/Game/BP/BP_Dashboard.unclampedRPM` _returnvalue_2 _asbp_dashboard)
    (elif (`self.isFuel`)
      (`PrimitiveComponent.SetMaterial` (`self.SM_Dial_Base`) 0 "/Game/Textures/Instances/MI_Dial_Fuel.MI_Dial_Fuel")
      (if (== (`self.fuelAmount`) 0.0)
        (set `/Game/BP/BP_Dashboard.fuelEmpty` true _asbp_dashboard)
        (else
          (bind _output_get_7 (set `self.fuelAmount` (- _fuelamount 0.001)))
          (`SceneComponent.K2_SetWorldRotation` _sm_dial (`KismetMathLibrary.MakeRotator` (`KismetMathLibrary.MapRangeClamped` _output_get_7 100.0 0.0 110.0 -110.0) _returnvalue_pitch _returnvalue_yaw) false false)
          (`TextRenderComponent.K2_SetText` (`self.TextRender`) (`KismetTextLibrary.Conv_Int64ToText` (`KismetMathLibrary.Round64` _fuelamount)))
          (set `/Game/BP/BP_Dashboard.fuelAmount` _fuelamount _asbp_dashboard)))
      (else
        (`PrimitiveComponent.SetMaterial` (`self.SM_Dial_Base`) 0 "/Game/Textures/Instances/MI_Dial_MPH.MI_Dial_MPH")
        (`SceneComponent.K2_SetWorldRotation` _sm_dial (`KismetMathLibrary.MakeRotator` (`KismetMathLibrary.MapRangeClamped` _returnvalue 0.0 160.0 -110.0 110.0) _returnvalue_pitch _returnvalue_yaw) false false)
        (`TextRenderComponent.K2_SetText` (`self.TextRender`) (`KismetTextLibrary.Conv_Int64ToText` (`KismetMathLibrary.Round64` _returnvalue)))))))

(fn `UserConstructionScript`)