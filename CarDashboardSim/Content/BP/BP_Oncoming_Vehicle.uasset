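; BP_Oncoming_Vehicle is a moving car actor that travels in a straight line and removes itself after a fixed lifetime.
; Each Tick sets the actor transform from the OncomingCar component's world transform, advancing it along the normalized Direction by Speed and delta time, without sweep.
; The component's yaw gets a fixed quarter-turn offset when applied to the actor.
; A Delay in the same Tick chain destroys the actor fifteen seconds after ticking starts.
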(event `self.ReceiveTick`
  (params (DeltaSeconds :type "Float (single-precision)"))
  (bind _returnvalue (`SceneComponent.K2_GetComponentToWorld` (`self.Oncoming Car`)))
  (`self.K2_SetActorTransform` (`KismetMathLibrary.MakeTransform` (+ (* (`KismetMathLibrary.Normal` (`self.Direction`)) (* (`GameplayStatics.GetWorldDeltaSeconds`) (`self.Speed`))) (.location _returnvalue)) (`KismetMathLibrary.MakeRotator` (.roll (.rotation _returnvalue)) (.pitch (.rotation _returnvalue)) (- (.yaw (.rotation _returnvalue)) 90.0)) (.scale _returnvalue)))
  (`KismetSystemLibrary.Delay` 15.0)
  (`self.K2_DestroyActor`))

(fn `UserConstructionScript`)