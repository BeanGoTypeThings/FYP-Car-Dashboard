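; PC_Simulation, a player controller by its prefix, handles the handoff between menu and car in a driving simulation.
; On BeginPlay it creates UI_Menu, switches it to its second page, sets UI-only input with a visible cursor and unpossesses the current pawn.
; The Re-PossessCar event possesses the stored CarRef if valid and flags the game as starting.
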(event `self.ReceiveBeginPlay`
  (bind _returnvalue (`|CreateWidget` "/Game/BP/GUI/UI_Menu.UI_Menu_C"))
  (`WidgetBlueprintLibrary.SetInputMode_UIOnlyEx` (`GameplayStatics.GetPlayerController` 0) null)
  (set `self.bShowMouseCursor` true)
  (`UserWidget.AddToViewport` _returnvalue 0)
  (`WidgetSwitcher.SetActiveWidgetIndex` (`/Game/BP/GUI/UI_Menu.WidgetSwitcher_421` _returnvalue) 1)
  (`self.UnPossess` (`GameplayStatics.GetPlayerController` 0)))

(event `Re-Possess Car`
  (bind _carref (`self.carRef`))
  (`/Engine/EditorBlueprintResources/StandardMacros.IsValid` _carref
    (:`Is Valid`
      (`self.Possess` (`GameplayStatics.GetPlayerController` 0) _carref)
      (set `self.isGameStarting` true))))

(fn `UserConstructionScript`)