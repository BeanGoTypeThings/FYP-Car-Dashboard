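; Drivable car pawn built on Character movement, with an animated steering wheel and five manual gears on number keys.
; Gears set acceleration and top speed, while Tick lowers ground friction as gear rises.
; Steering yaws the controller and front wheels in proportion to clamped forward speed, so it has no effect when stationary or reversing.
; Four side collision components only print debug hit messages.
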(event `EnhancedInput|/Game/BP/Input_Actions/IA_MoveBackwards`
  (params (ActionValue :type "Vector2D Structure") (ElapsedSeconds :type "Float (double-precision)") (TriggeredSeconds :type "Float (double-precision)") (InputAction :type "InputAction Object Reference" :default "/Game/BP/Input_Actions/IA_MoveBackwards.IA_MoveBackwards"))
  (bind (_returnvalue_roll _returnvalue_pitch _returnvalue_yaw) (`KismetMathLibrary.BreakRotator` (`self.GetControlRotation`)))
  (:`Triggered`
    (`self.AddMovementInput` (* (`KismetMathLibrary.GetForwardVector` (`KismetMathLibrary.MakeRotator` 0.0 0.0 _returnvalue_yaw)) -1.0) :!label _label))
  (:`Ongoing`
    (goto _label)))

(event `EnhancedInput|/Game/BP/Input_Actions/IA_MoveForward`
  (params (ActionValue :type "Vector2D Structure") (ElapsedSeconds :type "Float (double-precision)") (TriggeredSeconds :type "Float (double-precision)") (InputAction :type "InputAction Object Reference" :default "/Game/BP/Input_Actions/IA_MoveForward.IA_MoveForward"))
  (bind (_returnvalue_roll _returnvalue_pitch _returnvalue_yaw) (`KismetMathLibrary.BreakRotator` (`self.GetControlRotation`)))
  (:`Triggered`
    (`self.AddMovementInput` (`KismetMathLibrary.GetForwardVector` (`KismetMathLibrary.MakeRotator` 0.0 0.0 _returnvalue_yaw)) :!label _label_2))
  (:`Ongoing`
    (goto _label_2)))

(event `EnhancedInput|/Game/BP/Input_Actions/IA_MoveRight`
  (params (ActionValue :type "Float (double-precision)") (ElapsedSeconds :type "Float (double-precision)") (TriggeredSeconds :type "Float (double-precision)") (InputAction :type "InputAction Object Reference" :default "/Game/BP/Input_Actions/IA_MoveRight.IA_MoveRight"))
  (bind _steeringwheel (`self.SteeringWheel`))
  (bind (_returnvalue_roll _returnvalue_pitch _returnvalue_yaw) (`KismetMathLibrary.BreakRotator` (`SceneComponent.K2_GetComponentRotation` _steeringwheel)))
  (:`Triggered`
    (`self.AddControllerYawInput` (* (`self.Get Turn Velocity Normalised`) ActionValue 1.0))
    (`SceneComponent.K2_SetWorldRotation` _steeringwheel (`KismetMathLibrary.MakeRotator` (`KismetMathLibrary.FClamp` (- _returnvalue_roll (* ActionValue 2.5)) -540.0 540.0) _returnvalue_pitch _returnvalue_yaw) false false)))

(event `Key|One`
  (params (Key :type "Key Structure"))
  (bind _charactermovement (`self.CharacterMovement`))
  (:`Pressed`
    (set `self.gear` 1)
    (set `CharacterMovementComponent.MaxAcceleration` 50.0 _charactermovement)
    (set `CharacterMovementComponent.MaxWalkSpeed` 450.0 _charactermovement)))

(event `self.ReceiveTick`
  (params (DeltaSeconds :type "Float (single-precision)"))
  (bind _charactermovement (`self.CharacterMovement`))
  (`|ExecutionSequence`
    (:`then_0`
      (set `self.currentSpeed` (`KismetMathLibrary.VSizeXY` (`MovementComponent.Velocity` _charactermovement)))
      (switch `int` (`self.gear`)
        (:`1`
          (set `CharacterMovementComponent.GroundFriction` 8.0 _charactermovement))
        (:`2`
          (set `CharacterMovementComponent.GroundFriction` 7.0 _charactermovement))
        (:`3`
          (set `CharacterMovementComponent.GroundFriction` 4.0 _charactermovement))
        (:`4`
          (set `CharacterMovementComponent.GroundFriction` 2.0 _charactermovement))
        (:`5`
          (set `CharacterMovementComponent.GroundFriction` 1.0 _charactermovement))))
    (:`then_1`
      (`SceneComponent.K2_SetRelativeRotation` (`self.WheelFL`) (`KismetMathLibrary.MakeRotator` 0.0 0.0 (* (`|GetInputActionValue`) 45.0 (`self.Get Turn Velocity Normalised`))) false false)
      (`SceneComponent.K2_SetRelativeRotation` (`self.WheelFR`) (`KismetMathLibrary.MakeRotator` 0.0 0.0 (* (`|GetInputActionValue`) 45.0 (`self.Get Turn Velocity Normalised`))) false false))))

(event `self.Left Collision.OnComponentHit`
  (params (HitComponent :type "PrimitiveComponent Object Reference") (OtherActor :type "Actor Object Reference") (OtherComp :type "PrimitiveComponent Object Reference") (NormalImpulse :type "Vector Structure") (Hit :type "HitResult Structure (by ref)"))
  (`KismetSystemLibrary.PrintString` (`KismetStringLibrary.Concat_StrStr` (`KismetSystemLibrary.GetDisplayName` HitComponent) "LEFT")))

(event `Key|Two`
  (params (Key :type "Key Structure"))
  (bind _charactermovement (`self.CharacterMovement`))
  (:`Pressed`
    (set `self.gear` 2)
    (set `CharacterMovementComponent.MaxAcceleration` 100.0 _charactermovement)
    (set `CharacterMovementComponent.MaxWalkSpeed` 900.0 _charactermovement)))

(event `Key|Three`
  (params (Key :type "Key Structure"))
  (bind _charactermovement (`self.CharacterMovement`))
  (:`Pressed`
    (set `self.gear` 3)
    (set `CharacterMovementComponent.MaxAcceleration` 150.0 _charactermovement)
    (set `CharacterMovementComponent.MaxWalkSpeed` 1350.0 _charactermovement)))

(event `self.Right Collision.OnComponentHit`
  (params (HitComponent :type "PrimitiveComponent Object Reference") (OtherActor :type "Actor Object Reference") (OtherComp :type "PrimitiveComponent Object Reference") (NormalImpulse :type "Vector Structure") (Hit :type "HitResult Structure (by ref)"))
  (`KismetSystemLibrary.PrintString` (`KismetStringLibrary.Concat_StrStr` (`KismetSystemLibrary.GetDisplayName` HitComponent) "RIGHT")))

(event `Key|Four`
  (params (Key :type "Key Structure"))
  (bind _charactermovement (`self.CharacterMovement`))
  (:`Pressed`
    (set `self.gear` 4)
    (set `CharacterMovementComponent.MaxAcceleration` 200.0 _charactermovement)
    (set `CharacterMovementComponent.MaxWalkSpeed` 1800.0 _charactermovement)))

(event `self.Back Collision.OnComponentHit`
  (params (HitComponent :type "PrimitiveComponent Object Reference") (OtherActor :type "Actor Object Reference") (OtherComp :type "PrimitiveComponent Object Reference") (NormalImpulse :type "Vector Structure") (Hit :type "HitResult Structure (by ref)"))
  (`KismetSystemLibrary.PrintString` (`KismetStringLibrary.Concat_StrStr` (`KismetSystemLibrary.GetDisplayName` HitComponent) "BACK")))

(event `Key|Five`
  (params (Key :type "Key Structure"))
  (bind _charactermovement (`self.CharacterMovement`))
  (:`Pressed`
    (set `self.gear` 5)
    (set `CharacterMovementComponent.MaxAcceleration` 250.0 _charactermovement)
    (set `CharacterMovementComponent.MaxWalkSpeed` 2250.0 _charactermovement)))

(event `self.Front Collision.OnComponentHit`
  (params (HitComponent :type "PrimitiveComponent Object Reference") (OtherActor :type "Actor Object Reference") (OtherComp :type "PrimitiveComponent Object Reference") (NormalImpulse :type "Vector Structure") (Hit :type "HitResult Structure (by ref)"))
  (`KismetSystemLibrary.PrintString` (`KismetStringLibrary.Concat_StrStr` (`KismetSystemLibrary.GetDisplayName` HitComponent) "FRONT")))

(fn `Get Turn Velocity Normalised`
  (returns (ReturnValue :type "Float (double-precision)"))
  (return (`KismetMathLibrary.MapRangeClamped` (`KismetMathLibrary.Dot_VectorVector` (`self.GetVelocity`) (`self.GetActorForwardVector`)) 0.0 2250.0 0.0 1.0)))

(fn `UserConstructionScript`)